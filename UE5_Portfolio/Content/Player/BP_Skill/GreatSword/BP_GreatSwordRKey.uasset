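; Damage hitbox actor for the GreatSword R-key player skill.
; When its Box overlaps a Temp_Monster tagged Monster, it applies fixed damage through the monster's stat component OnAttacked, then switches the Box to the OverlapAll collision profile after a short delay.
; A Delay driven from Tick destroys the actor about two seconds after it starts ticking.
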(event `self.ReceiveTick`
  (params (DeltaSeconds :type "Float (single-precision)"))
  (`KismetSystemLibrary.Delay` 2.0)
  (`self.K2_DestroyActor`))

(event `self.Box.OnComponentBeginOverlap`
  (params (OverlappedComponent :type "PrimitiveComponent Object Reference") (OtherActor :type "Actor Object Reference") (OtherComp :type "PrimitiveComponent Object Reference") (OtherBodyIndex :type Integer) (bFromSweep :type Boolean) (SweepResult :type "HitResult Structure (by ref)"))
  (bind _astemp_monster (cast `/Game/Monster/Temp_Monster` OtherActor))
  (if (`self.ActorHasTag` OtherActor "Monster")
    (bind _returnvalue (`MeleeMonster.GetStatComp` _astemp_monster))
    (`MonsterStatComponent.OnAttacked` _returnvalue 45.0)
    (`KismetSystemLibrary.Delay` 0.5)
    (`PrimitiveComponent.SetCollisionProfileName` (`self.Box`) "OverlapAll" true)))

(fn `UserConstructionScript`)