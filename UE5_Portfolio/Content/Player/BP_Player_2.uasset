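; Player Blueprint that handles sword hit detection and the sword effect.
; When Box begins overlapping an actor tagged Monster during an attack, it casts to Temp_Monster and applies fixed damage through its stat component's OnAttacked.
; Tick activates SwordEffect every frame, passing NoneAttack as the Reset flag so the effect restarts whenever that returns true.
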(event `self.ReceiveTick`
  (params (DeltaSeconds :type "Float (single-precision)"))
  (bind _returnvalue (`self.NoneAttack`))
  (`ActorComponent.SetActive` (`self.SwordEffect`) true _returnvalue))

(event `self.Box.OnComponentBeginOverlap`
  (params (OverlappedComponent :type "PrimitiveComponent Object Reference") (OtherActor :type "Actor Object Reference") (OtherComp :type "PrimitiveComponent Object Reference") (OtherBodyIndex :type Integer) (bFromSweep :type Boolean) (SweepResult :type "HitResult Structure (by ref)"))
  (bind _returnvalue (`self.GetIsAttacking`))
  (if _returnvalue
    (if (`self.ActorHasTag` OtherActor "Monster")
      (bind _astemp_monster (cast `/Game/Monster/Temp_Monster` OtherActor))
      (bind _returnvalue_2 (`MeleeMonster.GetStatComp` _astemp_monster))
      (`MonsterStatComponent.OnAttacked` _returnvalue_2 4.0))))

(fn `UserConstructionScript`)